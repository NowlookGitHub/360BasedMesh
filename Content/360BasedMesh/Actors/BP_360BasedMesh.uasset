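; BP_360BasedMesh is an actor that displays an image on a sphere, set up entirely in the construction script.
; The BackfaceCulling flag selects an inversed or regular sphere mesh and also drives the material's show-inside-sphere parameter.
; A dynamic instance of M_360BasedMesh receives the image, mirroring, vertical scale and offset, and top and bottom crop with a crop color.
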(fn `InitMaterial`
  (bind _returnvalue (`KismetMaterialLibrary.CreateDynamicMaterialInstance` "/Game/360BasedMesh/Materials/M_360BasedMesh.M_360BasedMesh"))
  (bind _output_get (set `self.MeshMaterial` _returnvalue))
  (`PrimitiveComponent.SetMaterial` (`self.StaticMesh`) 0 _output_get))

(fn `InitMesh`
  (`StaticMeshComponent.SetStaticMesh` (`self.StaticMesh`) (select `bool` (`self.bBackfaceCulling`) :`false` "/Game/360BasedMesh/Meshes/SM_Sphere.SM_Sphere" :`true` "/Game/360BasedMesh/Meshes/SM_InversedSphere.SM_InversedSphere" :!type "StaticMesh Object Reference")))

(fn `UpdateMaterialParameters`
  (bind _meshmaterial (`self.MeshMaterial`))
  (`MaterialInstanceDynamic.SetVectorParameterValue` _meshmaterial "CropColor" (`self.CropColor`))
  (`MaterialInstanceDynamic.SetTextureParameterValue` _meshmaterial "Image" (`self.Image`))
  (`MaterialInstanceDynamic.SetScalarParameterValue` _meshmaterial "bMirrorImage" (`KismetMathLibrary.Conv_BoolToDouble` (`self.bMirrorImage`)))
  (`MaterialInstanceDynamic.SetScalarParameterValue` _meshmaterial "bShowImageInsideTheSphere" (`KismetMathLibrary.Conv_BoolToDouble` (`self.bBackfaceCulling`)))
  (`MaterialInstanceDynamic.SetScalarParameterValue` _meshmaterial "YScale" (`self.YScale`))
  (`MaterialInstanceDynamic.SetScalarParameterValue` _meshmaterial "YOffset" (`self.YOffset`))
  (`MaterialInstanceDynamic.SetScalarParameterValue` _meshmaterial "BottomCrop" (`self.BottomCrop`))
  (`MaterialInstanceDynamic.SetScalarParameterValue` _meshmaterial "TopCrop" (`self.TopCrop`)))

(fn `UserConstructionScript`
  (`self.InitMesh`)
  (`self.InitMaterial`)
  (`self.UpdateMaterialParameters`))